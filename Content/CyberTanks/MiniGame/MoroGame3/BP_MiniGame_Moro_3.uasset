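; Third Moro mini-game Blueprint in CyberTanks, where overlap boxes decide success or failure.
; A restarting timeline (OśCzasu) drives MovingCUbe along its local X axis, scaled by Speed.
; IA_Move pitches PlayerMoveLeft by sensitivity-scaled input, clamped to a half-turn range.
; Box1 calls Fail when Kula (ball) enters, while Box, Box2 and Box3 call Success for components tagged "K".
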(event `self.ReceiveBeginPlay`
  (bind (_direction _newtrack_0) (`Timeline|Oś czasu` :!via `PlayFromStart` :!label _label)
    (:`Update`
      (`SceneComponent.K2_AddLocalOffset` (`self.MovingCUbe`) (`KismetMathLibrary.MakeVector` (* (`self.Speed`) _newtrack_0)) false false))
    (:`Finished`
      (goto _label :!via `PlayFromStart`))))

(event `self.Box1.OnComponentBeginOverlap`
  (params (OverlappedComponent :type "PrimitiveComponent Object Reference") (OtherActor :type "Actor Object Reference") (OtherComp :type "PrimitiveComponent Object Reference") (OtherBodyIndex :type Integer) (bFromSweep :type Boolean) (SweepResult :type "HitResult Structure (by ref)"))
  (if (== OtherComp (`self.Kula`))
    (`self.Fail`)))

(event `EnhancedInput|/Game/ThirdPerson/Input/Actions/IA_Move`
  (params (ActionValue :type "Vector2D Structure") (ElapsedSeconds :type "Float (double-precision)") (TriggeredSeconds :type "Float (double-precision)") (InputAction :type "InputAction Object Reference" :default "/Game/ThirdPerson/Input/Actions/IA_Move.IA_Move"))
  (bind _returnvalue_x (`KismetMathLibrary.BreakVector2D` (`KismetMathLibrary.Normal2D` ActionValue)))
  (bind _playermoveleft (`self.PlayerMoveLeft`))
  (bind (_relativerotation_roll _relativerotation_pitch _relativerotation_yaw) (`KismetMathLibrary.BreakRotator` (`SceneComponent.RelativeRotation` _playermoveleft)))
  (:`Triggered`
    (`SceneComponent.K2_AddRelativeRotation` (`self.PlayerMoveLeft`) (`KismetMathLibrary.MakeRotator` 0.0 (* _returnvalue_x (`self.Sensivity`))) false false)
    (`SceneComponent.K2_SetRelativeRotation` _playermoveleft (`KismetMathLibrary.MakeRotator` _relativerotation_roll (`KismetMathLibrary.FClamp` _relativerotation_pitch -90.0 90.0) _relativerotation_yaw) false false)))

(event `self.Box2.OnComponentBeginOverlap`
  (params (OverlappedComponent :type "PrimitiveComponent Object Reference") (OtherActor :type "Actor Object Reference") (OtherComp :type "PrimitiveComponent Object Reference") (OtherBodyIndex :type Integer) (bFromSweep :type Boolean) (SweepResult :type "HitResult Structure (by ref)"))
  (if (`ActorComponent.ComponentHasTag` OtherComp "K")
    (`self.Success`)))

(event `self.Box.OnComponentBeginOverlap`
  (params (OverlappedComponent :type "PrimitiveComponent Object Reference") (OtherActor :type "Actor Object Reference") (OtherComp :type "PrimitiveComponent Object Reference") (OtherBodyIndex :type Integer) (bFromSweep :type Boolean) (SweepResult :type "HitResult Structure (by ref)"))
  (if (`ActorComponent.ComponentHasTag` OtherComp "K")
    (`self.Success`)))

(event `self.Box3.OnComponentBeginOverlap`
  (params (OverlappedComponent :type "PrimitiveComponent Object Reference") (OtherActor :type "Actor Object Reference") (OtherComp :type "PrimitiveComponent Object Reference") (OtherBodyIndex :type Integer) (bFromSweep :type Boolean) (SweepResult :type "HitResult Structure (by ref)"))
  (if (`ActorComponent.ComponentHasTag` OtherComp "K")
    (`self.Success`)))

(fn `UserConstructionScript`
  (`parent.UserConstructionScript`))